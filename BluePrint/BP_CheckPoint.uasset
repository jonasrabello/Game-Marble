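; Checkpoint actor for a marble game that either updates the marble's reset point or ends the run.
; Every Tick it polls its Box for an overlapping BP_Marble, then passes its Position to the first marble found in the level.
; When flagged FinalPosition, it instead clears widgets, shows WD_PlayAgain with the mouse cursor, and clears the flag so the screen is created once.
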(event `self.ReceiveTick`
  (params (DeltaSeconds :type "Float (single-precision)"))
  (if (> (`KismetArrayLibrary.Array_Length` (`PrimitiveComponent.GetOverlappingActors` (`self.Box`) "/Game/Project2/BluePrint/BP_Marble.BP_Marble_C")) 0)
    (if (`self.FinalPosition`)
      (`self.CallPlayAgain`)
      (else
        (bind _outactors (`GameplayStatics.GetAllActorsOfClass` "/Game/Project2/BluePrint/BP_Marble.BP_Marble_C"))
        (`Marble.SetResetPosition` (`|GetArrayItem` _outactors) (`self.Position`))))))

(event `CallPlayAgain`
  (`WidgetLayoutLibrary.RemoveAllWidgets`)
  (bind _returnvalue (`|CreateWidget` "/Game/Project2/UI/WD_PlayAgain.WD_PlayAgain_C" (`GameplayStatics.GetPlayerController` 0)))
  (`UserWidget.AddToViewport` _returnvalue 0)
  (`WidgetBlueprintLibrary.SetInputMode_GameAndUIEx` (`GameplayStatics.GetPlayerController` 0) _returnvalue)
  (set `PlayerController.bShowMouseCursor` true (`GameplayStatics.GetPlayerController` 0))
  (set `self.FinalPosition` false))

(fn `UserConstructionScript`)