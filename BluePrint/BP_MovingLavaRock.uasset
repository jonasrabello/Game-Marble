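; BP_MovingLavaRock is a moving lava rock hazard that damages the marble on contact.
; Tick starts a round trip whenever the rock sits at StartPoint, chaining two MoveComponentTo calls to EndPoint and back.
; A hit on BP_Marble deals damage, then a WasHit flag blocks further hits for a one-second delay.
; The burn sound plays according to the marble's own collision sound toggle and volume.
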(event `self.ReceiveBeginPlay`)

(event `self.ReceiveTick`
  (params (DeltaSeconds :type "Float (single-precision)"))
  (bind _returnvalue (`SceneComponent.GetRelativeTransform` (`self.Rock`)))
  (bind _returnvalue_2 (`KismetMathLibrary.TransformRotation` _returnvalue))
  (if (== (`KismetMathLibrary.TransformLocation` _returnvalue) (`self.StartPoint`))
    (`KismetSystemLibrary.MoveComponentTo` (`self.Rock`) (`self.EndPoint`) _returnvalue_2 false false (`self.OverTime`))
    (`KismetSystemLibrary.MoveComponentTo` (`self.Rock`) (`self.StartPoint`) _returnvalue_2 false false (`self.OverTime`))))

(event `self.ReceiveHit`
  (params (MyComp :type "PrimitiveComponent Object Reference") (Other :type "Actor Object Reference") (OtherComp :type "PrimitiveComponent Object Reference") (bSelfMoved :type Boolean) (HitLocation :type "Vector Structure") (HitNormal :type "Vector Structure") (NormalImpulse :type "Vector Structure") (Hit :type "HitResult Structure (by ref)"))
  (bind _asbp_marble (cast `/Game/Project2/BluePrint/BP_Marble` Other))
  (if (not (`self.WasHit`))
    (`Marble.MarbleTakeDamage` _asbp_marble (`self.DamagePoints`))
    (set `self.WasHit` true)
    (`self.CheckEffects` _asbp_marble)
    (if (`self.PlayCollision`)
      (`GameplayStatics.PlaySound2D` "/Game/ProjectAssets/Sounds/burned.burned" (`self.Volume`)))
    (`KismetSystemLibrary.Delay` 1.0)
    (set `self.WasHit` false)))

(event `CheckEffects`
  (params (Marble :type "/Game/Project2/BluePrint/BP_Marble Object Reference"))
  (set `self.PlayCollision` (`Marble.playCollision` Marble))
  (set `self.Volume` (`Marble.collisionSoundVolume` Marble)))

(fn `UserConstructionScript`)