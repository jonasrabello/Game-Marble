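; BP_Fence is an obstacle actor that damages a BP_Marble when the marble hits it.
; On Hit it applies DamagePoint via MarbleTakeDamage, then copies the marble's collision-sound flag and volume to decide whether to play a 2D wooden thud.
; A WasHit flag, cleared after a one-second delay, debounces repeated hits and is shared across all marbles.
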(event `self.ReceiveBeginPlay`)

(event `self.ReceiveHit`
  (params (MyComp :type "PrimitiveComponent Object Reference") (Other :type "Actor Object Reference") (OtherComp :type "PrimitiveComponent Object Reference") (bSelfMoved :type Boolean) (HitLocation :type "Vector Structure") (HitNormal :type "Vector Structure") (NormalImpulse :type "Vector Structure") (Hit :type "HitResult Structure (by ref)"))
  (bind _asbp_marble (cast `/Game/Project2/BluePrint/BP_Marble` Other))
  (if (not (`self.WasHit`))
    (`Marble.MarbleTakeDamage` _asbp_marble (`self.DamagePoint`))
    (set `self.WasHit` true)
    (`self.CheckEffects` _asbp_marble)
    (if (`self.PlayCollision`)
      (`GameplayStatics.PlaySound2D` "/Game/ProjectAssets/Sounds/thud_on_woode.thud_on_woode" (`self.Volume`)))
    (`KismetSystemLibrary.Delay` 1.0)
    (set `self.WasHit` false)))

(event `CheckEffects`
  (params (Marble :type "/Game/Project2/BluePrint/BP_Marble Object Reference"))
  (set `self.PlayCollision` (`Marble.playCollision` Marble))
  (set `self.Volume` (`Marble.collisionSoundVolume` Marble)))

(fn `UserConstructionScript`)