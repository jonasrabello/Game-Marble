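; BP_WoodFloor is a moving wooden platform that carries a marble, shuttling between StartPoint and EndPoint.
; Tick detects marbles through Box and gates movement on a linked OtherWoodFloor, pausing new moves while that floor's marble is in transit.
; Cubes act as toggleable blockers, varying by Type: a loaded floor stops at the end and drops its own, while the linked floor's arrival opens others.
; ResetBox restores position and blockers.
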(event `self.ReceiveBeginPlay`
  (`self.SetBeginStatus`)
  (`self.HideAdditionalCube`))

(event `SetBeginStatus`
  (bind _cube5 (`self.Cube5`))
  (bind _cube3 (`self.Cube3`))
  (if (`KismetStringLibrary.EqualEqual_StrStr` (`self.Type`) "A")
    (`SceneComponent.SetHiddenInGame` _cube3 true false)
    (`PrimitiveComponent.SetCollisionEnabled` _cube3 "NoCollision")
    (`SceneComponent.SetHiddenInGame` _cube5 true false)
    (`PrimitiveComponent.SetCollisionEnabled` _cube5 "NoCollision")))

(event `HideAdditionalCube`
  (bind _cube6 (`self.Cube6`))
  (if (not (`self.additionCube`))
    (`SceneComponent.SetHiddenInGame` _cube6 true false)
    (`PrimitiveComponent.SetCollisionEnabled` _cube6 "NoCollision")))

(event `ShowAdditionalCube`
  (bind _cube6 (`self.Cube6`))
  (if (`self.additionCube`)
    (`SceneComponent.SetHiddenInGame` _cube6 false false)
    (`PrimitiveComponent.SetCollisionEnabled` _cube6 "QueryAndPhysics")))

(event `self.ReceiveActorBeginOverlap`
  (params (OtherActor :type "Actor Object Reference")))

(event `self.ReceiveTick`
  (params (DeltaSeconds :type "Float (single-precision)"))
  (`|ExecutionSequence`
    (:`then_0`
      (`self.CheckMarble`))
    (:`then_1`
      (if (!= (`self.OtherWoodFloor`) self)
        (if (`/BluePrint/BP_WoodFloor.ContainMarble` (`self.OtherWoodFloor`))
          (if (`/BluePrint/BP_WoodFloor.End` (`self.OtherWoodFloor`))
            (`self.Move`))
          (else
            (`self.Move`)))
        (else
          (`self.Move`))))))

(event `CheckMarble`
  (if (`self.ContainMarble`)
    _
    (elif (> (`KismetArrayLibrary.Array_Length` (`PrimitiveComponent.GetOverlappingActors` (`self.Box`) "/Game/Project2/BluePrint/BP_Marble.BP_Marble_C")) 0)
      (set `self.ContainMarble` true))))

(event `Move`
  ;[1 1 1] Move wooden floor back and forward
  (`|ExecutionSequence`
    (:`then_0`
      (`self.DestroyCube3`)
      (`self.DestroyCube5`))
    (:`then_1`
      (if (== (`KismetMathLibrary.TransformLocation` (`SceneComponent.GetRelativeTransform` (`self.Cube`))) (`self.StartPoint`))
        (`|ExecutionSequence`
          (:`then_0`
            (set `self.End` false))
          (:`then_1`
            (`KismetSystemLibrary.Delay` (`self.Delay`))
            (`KismetSystemLibrary.MoveComponentTo` (`self.Cube`) (`self.EndPoint`) (struct) false false (`self.OverTime`))
            (`|ExecutionSequence`
              (:`then_0`
                (set `self.End` true))
              (:`then_1`
                (if (`self.ContainMarble`)
                  (`self.DestroyCube4`)
                  (else
                    (`KismetSystemLibrary.Delay` (`self.Delay`))
                    (`KismetSystemLibrary.MoveComponentTo` (`self.Cube`) (`self.StartPoint`) (struct) false false (`self.OverTime`))))))))))))

(event `DestroyCube3`
  (bind _cube3 (`self.Cube3`))
  (if (`/BluePrint/BP_WoodFloor.ContainMarble` (`self.OtherWoodFloor`))
    (if (`/BluePrint/BP_WoodFloor.End` (`self.OtherWoodFloor`))
      (`SceneComponent.SetHiddenInGame` _cube3 true true)
      (`PrimitiveComponent.SetCollisionEnabled` _cube3 "NoCollision"))))

(event `DestroyCube4`
  (bind _cube4 (`self.Cube4`))
  (bind _cube6 (`self.Cube6`))
  (`SceneComponent.SetHiddenInGame` _cube4 true false)
  (`PrimitiveComponent.SetCollisionEnabled` _cube4 "NoCollision")
  (`SceneComponent.SetHiddenInGame` _cube6 true false)
  (`PrimitiveComponent.SetCollisionEnabled` _cube6 "NoCollision"))

(event `DestroyCube5`
  (bind _cube5 (`self.Cube5`))
  (if (`/BluePrint/BP_WoodFloor.ContainMarble` (`self.OtherWoodFloor`))
    (if (`/BluePrint/BP_WoodFloor.End` (`self.OtherWoodFloor`))
      (`SceneComponent.SetHiddenInGame` _cube5 true false)
      (`PrimitiveComponent.SetCollisionEnabled` _cube5 "NoCollision"))))

(event `ResetBox`
  (set `self.ContainMarble` false)
  (set `self.End` false)
  (`self.SetCube3`)
  (`self.SetCube4`)
  (`self.SetCube5`)
  (`self.ResetBoxPosition`))

(event `ResetBoxPosition`
  (if (!= (`KismetMathLibrary.TransformLocation` (`SceneComponent.GetRelativeTransform` (`self.Cube`))) (`self.StartPoint`))
    (`KismetSystemLibrary.MoveComponentTo` (`self.Cube`) (`self.StartPoint`) (struct) false false 0.0)))

(event `SetCube3`
  (bind _cube3 (`self.Cube3`))
  (if (`KismetStringLibrary.EqualEqual_StrStr` (`self.Type`) "B")
    (`SceneComponent.SetHiddenInGame` _cube3 false true)
    (`PrimitiveComponent.SetCollisionEnabled` _cube3 "QueryAndPhysics")))

(event `SetCube4`
  (bind _cube4 (`self.Cube4`))
  (`SceneComponent.SetHiddenInGame` _cube4 false false)
  (`PrimitiveComponent.SetCollisionEnabled` _cube4 "QueryAndPhysics")
  (`self.ShowAdditionalCube`))

(event `SetCube5`
  (bind _cube5 (`self.Cube5`))
  (if (`KismetStringLibrary.EqualEqual_StrStr` (`self.Type`) "B")
    (`SceneComponent.SetHiddenInGame` _cube5 false false)
    (`PrimitiveComponent.SetCollisionEnabled` _cube5 "QueryAndPhysics")))

(fn `UserConstructionScript`)